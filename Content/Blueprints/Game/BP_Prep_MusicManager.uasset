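; Music manager that turns live MIDI input into MetaSound playback on a Quartz clock.
; BeginPlay starts the clock, a bar-quantized, BPM-fed bass drum and quarter-note UI pulses, then binds MIDI devices by index to four handlers.
; Controller 1 plays a polyphonic synth via note-indexed voices, controller 2 triggers sixteenth-quantized drum samples, and 3 and 4 only print.
; Helper functions list devices, assign them to slots by name and clear slots.
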(event `self.ReceiveBeginPlay`
  (bind _returnvalue (`QuartzSubsystem.CreateNewClock` :`self` (subsystem `QuartzSubsystem`) :`ClockName` "MainClock"))
  (bind _output_get (set `self.MainClock` _returnvalue))
  (bind _clockhandle (`QuartzClockHandle.SetBeatsPerMinute` :`self` _output_get :`BeatsPerMinute` (`self.Beats Per Minute`)))
  (bind _clockhandle_2 (`QuartzClockHandle.StartClock` _clockhandle))
  (`QuartzClockHandle.SubscribeToQuantizationEvent` _clockhandle_2 "QuarterNote" (`|CreateDelegate` :!event `On4thBeat`))
  (`self.AddAllInitialController`)
  (bind _returnvalue_2 (`GameplayStatics.CreateSound2D` "/Game/Prep/Metasound/MSS_Bassdrum.MSS_Bassdrum" 1.0 1.0 0.0 null))
  (`AudioParameterControllerInterface.SetFloatParameter` _returnvalue_2 "BPM" (`self.Beats Per Minute`))
  (`AudioComponent.PlayQuantized` :`self` _returnvalue_2 :`InClockHandle` (`self.MainClock`) :`InQuantizationBoundary` (make `QuartzQuantizationBoundary` "Bar" 1.0 "CurrentTimeRelative")))

(event `Controller1_Event`
  (params (MIDIDeviceController :type "MIDIDeviceController Object Reference") (Timestamp :type Integer) (EventType :type "EMIDIEventType Enum" :default "Unknown") (Channel :type Integer) (ControlID :type Integer) (Velocity :type Integer) (RawEventType :type Integer))
  (bind _controller1voicearray (`self.Controller1VoiceArray`))
  (`KismetSystemLibrary.PrintString` (`KismetTextLibrary.Conv_TextToString` (`|FormatText` "CONTROLLER 1 {CC} {Value}" ControlID Velocity)) true true (struct :`G` 0.66 :`B` 1.0 :`A` 1.0) 2.0 "Controller1")
  (switch `EMIDIEventType` EventType
    (:`NoteOff`
      ; Play polyphonic Synth
      (`AudioParameterControllerInterface.SetTriggerParameter` (`|GetArrayItem` _controller1voicearray ControlID) "Trigger Release"))
    (:`NoteOn`
      (bind _returnvalue (`GameplayStatics.CreateSound2D` "/Game/Prep/Metasound/MSS_AdditiveSynth.MSS_AdditiveSynth" 1.0 1.0 0.0 null))
      (`KismetArrayLibrary.Array_Set` _controller1voicearray ControlID _returnvalue true)
      (`AudioParameterControllerInterface.SetFloatParameter` _returnvalue "MIDI In" (`KismetMathLibrary.Conv_IntToDouble` ControlID))
      (`AudioComponent.Play` _returnvalue 0.0))))

(event `Controller2_Event`
  (params (MIDIDeviceController :type "MIDIDeviceController Object Reference") (Timestamp :type Integer) (EventType :type "EMIDIEventType Enum" :default "Unknown") (Channel :type Integer) (ControlID :type Integer) (Velocity :type Integer) (RawEventType :type Integer))
  (`KismetSystemLibrary.PrintString` (`KismetTextLibrary.Conv_TextToString` (`|FormatText` "CONTROLLER 2  {CC} {Value}" ControlID Velocity)) true true (struct :`R` 1.0 :`B` 0.113278 :`A` 1.0) 2.0 "Controller2")
  (switch `EMIDIEventType` EventType
    (:`NoteOn`
      (bind _returnvalue (`GameplayStatics.CreateSound2D` "/Game/Prep/Metasound/MSS_DrumSampler.MSS_DrumSampler" 1.0 1.0 0.0 null))
      (switch `string` (`KismetStringLibrary.Conv_IntToString` ControlID)
        (:`36`
          (`AudioComponent.SetWaveParameter` _returnvalue "Wave Asset" "/Game/Prep/Samples/DrumSamples/Kick_10.Kick_10"))
        (:`38`
          (`AudioComponent.SetWaveParameter` _returnvalue "Wave Asset" "/Game/Prep/Samples/DrumSamples/Snare_13.Snare_13"))
        (:`40`
          (`AudioComponent.SetWaveParameter` _returnvalue "Wave Asset" "/Game/Prep/Samples/Calabasa01.Calabasa01"))
        (:`41`
          (`AudioComponent.SetWaveParameter` _returnvalue "Wave Asset" "/Game/Prep/Samples/Calabasa02.Calabasa02"))
        (:`43`
          (`AudioComponent.SetWaveParameter` _returnvalue "Wave Asset" "/Game/Prep/Samples/DrumSamples/Hi_Hat_27.Hi_Hat_27"))
        (:`45`
          (`AudioComponent.SetWaveParameter` _returnvalue "Wave Asset" "/Game/Metasound/Samples/Voix01.Voix01"))
        (:`47`
          (`AudioComponent.SetWaveParameter` _returnvalue "Wave Asset" "/Game/Prep/Samples/Voix02.Voix02"))
        (:`48`
          (`AudioComponent.SetWaveParameter` _returnvalue "Wave Asset" "/Game/Metasound/Samples/Voix03.Voix03")))
      (`AudioComponent.PlayQuantized` :`self` _returnvalue :`InClockHandle` (`self.MainClock`) :`InQuantizationBoundary` (make `QuartzQuantizationBoundary` "SixteenthNote" 1.0 "CurrentTimeRelative")))))

(event `Controller3_Event`
  (params (MIDIDeviceController :type "MIDIDeviceController Object Reference") (Timestamp :type Integer) (EventType :type "EMIDIEventType Enum" :default "Unknown") (Channel :type Integer) (ControlID :type Integer) (Velocity :type Integer) (RawEventType :type Integer))
  (`KismetSystemLibrary.PrintString` (`KismetTextLibrary.Conv_TextToString` (`|FormatText` "CONTROLLER 3 {CC} {Value}" ControlID Velocity)) true true (struct :`R` 1.0 :`G` 0.492826 :`A` 1.0) 2.0 "Controller3"))

(event `Controller4_Event`
  (params (MIDIDeviceController :type "MIDIDeviceController Object Reference") (Timestamp :type Integer) (EventType :type "EMIDIEventType Enum" :default "Unknown") (Channel :type Integer) (ControlID :type Integer) (Velocity :type Integer) (RawEventType :type Integer))
  (`KismetSystemLibrary.PrintString` (`KismetTextLibrary.Conv_TextToString` (`|FormatText` "CONTROLLER 4 {CC} {Value}" ControlID Velocity)) true true (struct :`R` 0.02943 :`G` 1.0 :`B` 0.744557 :`A` 1.0) 2.0 "Controller4"))

(event `On4thBeat`
  (params (ClockName :type Name) (QuantizationType :type "EQuartzCommandQuantization Enum" :default "Bar") (NumBars :type Integer) (Beat :type Integer) (BeatFraction :type "Float (single-precision)"))
  (bind _asbp_edm1507_player_controller (cast `/Game/Blueprints/Game/BP_EDM1507_PlayerController` (`GameplayStatics.GetPlayerController` 0)))
  (bind _mainui (`/Game/Blueprints/Game/BP_EDM1507_PlayerController.MainUI` _asbp_edm1507_player_controller))
  (`UserWidget.PlayAnimation` _mainui (`/Game/Blueprints/UI/W_MainUI.Beat` _mainui) 0.0 1 "Forward" 1.0 false))

(fn `AddAllInitialController`
  (`KismetArrayLibrary.Array_Clear` (`self.InitialControllerArray`))
  (bind _outmididevices (`MIDIDeviceManager.FindMIDIDevices`))
  (for (_array_element _array_index) _outmididevices
    (bind (_deviceid _devicename _bcanreceivefrom) (break `FoundMIDIDevice` _array_element))
    (if _bcanreceivefrom
      (bind _returnvalue (`MIDIDeviceManager.CreateMIDIDeviceController` _deviceid))
      (`KismetArrayLibrary.Array_Add` (`self.InitialControllerArray`) _returnvalue)
      (switch `int` _array_index
        (:`1`
          (add `MIDIDeviceController.OnMIDIEvent` _returnvalue (`|CreateDelegate` :!event `Controller1_Event`)))
        (:`2`
          (add `MIDIDeviceController.OnMIDIEvent` _returnvalue (`|CreateDelegate` :!event `Controller2_Event`)))
        (:`3`
          (add `MIDIDeviceController.OnMIDIEvent` _returnvalue (`|CreateDelegate` :!event `Controller3_Event`)))
        (:`4`
          (add `MIDIDeviceController.OnMIDIEvent` _returnvalue (`|CreateDelegate` :!event `Controller4_Event`))))))
  (return))

(fn `AddController`
  (params (Name :type String) (NewID :type String))
  (bind _founddevicesnames (`self.FindAllDevices`))
  (for (_array_element _array_index) _founddevicesnames
    (if (`KismetStringLibrary.EqualEqual_StrStr` _array_element Name)
      (bind _output (`|GetArrayItem` (`self.InitialControllerArray`) _array_index))
      (`/Engine/EditorBlueprintResources/StandardMacros.IsValid` _output
        (:`Is Valid`
          (clear `MIDIDeviceController.OnMIDIEvent` _output)
          (switch `int` (`KismetStringLibrary.Conv_StringToInt` NewID)
            (:`1`
              (bind _output_get (set `self.MIDIController01` _output))
              (add `MIDIDeviceController.OnMIDIEvent` _output_get (`|CreateDelegate` :!event `Controller1_Event`)))
            (:`2`
              (bind _output_get_2 (set `self.MIDIController02` _output))
              (add `MIDIDeviceController.OnMIDIEvent` _output_get_2 (`|CreateDelegate` :!event `Controller2_Event`)))
            (:`3`
              (bind _output_get_3 (set `self.MIDIController03` _output))
              (add `MIDIDeviceController.OnMIDIEvent` _output_get_3 (`|CreateDelegate` :!event `Controller3_Event`)))
            (:`4`
              (bind _output_get_4 (set `self.MIDIController04` _output))
              (add `MIDIDeviceController.OnMIDIEvent` _output_get_4 (`|CreateDelegate` :!event `Controller4_Event`)))))
        (:`Is Not Valid`
          (`KismetSystemLibrary.PrintString` "INVALID CONTROLLER" true true (struct :`R` 1.0 :`B` 0.022252 :`A` 1.0)))))))

(fn `ClearAllDevices`
  (bind _midicontroller01 (`self.MIDIController01`))
  (bind _midicontroller02 (`self.MIDIController02`))
  (bind _midicontroller03 (`self.MIDIController03`))
  (bind _midicontroller04 (`self.MIDIController04`))
  (`|ExecutionSequence`
    (:`then_0`
      (`/Engine/EditorBlueprintResources/StandardMacros.IsValid` _midicontroller01
        (:`Is Valid`
          (clear `MIDIDeviceController.OnMIDIEvent` _midicontroller01)
          (set `self.MIDIController01` null))))
    (:`then_1`
      (`/Engine/EditorBlueprintResources/StandardMacros.IsValid` _midicontroller02
        (:`Is Valid`
          (clear `MIDIDeviceController.OnMIDIEvent` _midicontroller02)
          (set `self.MIDIController02` null))))
    (:`then_2`
      (`/Engine/EditorBlueprintResources/StandardMacros.IsValid` _midicontroller03
        (:`Is Valid`
          (clear `MIDIDeviceController.OnMIDIEvent` _midicontroller03)
          (set `self.MIDIController03` null))))
    (:`then_3`
      (`/Engine/EditorBlueprintResources/StandardMacros.IsValid` _midicontroller04
        (:`Is Valid`
          (clear `MIDIDeviceController.OnMIDIEvent` _midicontroller04)
          (set `self.MIDIController04` null))))
    (:`then_4`
      (return))))

(fn `FindAllDevices`
  (returns (FoundDevicesNames :type "Array of String"))
  (locals (DevicesNames :type "Array of String"))
  (bind _outmididevices (`MIDIDeviceManager.FindMIDIDevices`))
  (for _array_element _outmididevices
    (bind (_deviceid _devicename _bcanreceivefrom) (break `FoundMIDIDevice` _array_element))
    (if _bcanreceivefrom
      (bind _returnvalue (`MIDIDeviceManager.CreateMIDIDeviceController` _deviceid))
      (`KismetArrayLibrary.Array_Add` (`local.DevicesNames`) (`KismetTextLibrary.Conv_TextToString` (`|FormatText` "{DeviceID} {Name}" _deviceid _devicename)))
      (`KismetArrayLibrary.Array_Add` (`self.InitialControllerArray`) _returnvalue)))
  (return (`local.DevicesNames`)))

(fn `UserConstructionScript`)