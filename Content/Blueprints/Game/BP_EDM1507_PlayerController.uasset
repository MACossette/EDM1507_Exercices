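; Player controller for the EDM1507 project that turns the keyboard into a simple MetaSound synth instrument.
; On BeginPlay it prints a debug message, shows the mouse cursor and adds W_MainUI to the viewport.
; Space plays MSS_Synth01, while A, S, D and F each start their own MSS_AdditiveSynth note (C, E, G, B) through the "MIDI In" parameter.
; Releasing a note key fires that sound's "Trigger Release" trigger.
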(event `self.ReceiveBeginPlay`
  (`KismetSystemLibrary.PrintString` "Je suis BP_EDM1507_PlayerController" true true (struct :`R` 1.0 :`B` 0.784622 :`A` 1.0) 100.0)
  (set `self.bShowMouseCursor` true)
  (bind _returnvalue (`|CreateWidget` "/Game/Blueprints/UI/W_MainUI.W_MainUI_C"))
  (bind _output_get (set `self.MainUI` _returnvalue))
  (`UserWidget.AddToViewport` _output_get 0))

(event `Key|SpaceBar`
  (params (Key :type "Key Structure"))
  (:`Pressed`
    (bind _returnvalue (`GameplayStatics.CreateSound2D` "/Game/Metasound/MSS_Synth01.MSS_Synth01" 1.0 1.0 0.0 null))
    (`AudioComponent.Play` _returnvalue 0.0)))

(event `Key|A`
  (params (Key :type "Key Structure"))
  (:`Pressed`
    (bind _returnvalue (`GameplayStatics.CreateSound2D` "/Game/Prep/Metasound/MSS_AdditiveSynth.MSS_AdditiveSynth" 1.0 1.0 0.0 null))
    (bind _output_get (set `self.AdditiveC` _returnvalue))
    (`AudioParameterControllerInterface.SetFloatParameter` _output_get "MIDI In" 60.0)
    (`AudioComponent.Play` (`self.AdditiveC`) 0.0))
  (:`Released`
    (`AudioParameterControllerInterface.SetTriggerParameter` (`self.AdditiveC`) "Trigger Release")))

(event `Key|S`
  (params (Key :type "Key Structure"))
  (:`Pressed`
    (bind _returnvalue (`GameplayStatics.CreateSound2D` "/Game/Prep/Metasound/MSS_AdditiveSynth.MSS_AdditiveSynth" 1.0 1.0 0.0 null))
    (bind _output_get (set `self.AdditiveE` _returnvalue))
    (`AudioParameterControllerInterface.SetFloatParameter` _output_get "MIDI In" 64.0)
    (`AudioComponent.Play` (`self.AdditiveE`) 0.0))
  (:`Released`
    (`AudioParameterControllerInterface.SetTriggerParameter` (`self.AdditiveE`) "Trigger Release")))

(event `Key|D`
  (params (Key :type "Key Structure"))
  (:`Pressed`
    (bind _returnvalue (`GameplayStatics.CreateSound2D` "/Game/Prep/Metasound/MSS_AdditiveSynth.MSS_AdditiveSynth" 1.0 1.0 0.0 null))
    (bind _output_get (set `self.AdditiveG` _returnvalue))
    (`AudioParameterControllerInterface.SetFloatParameter` _output_get "MIDI In" 67.0)
    (`AudioComponent.Play` (`self.AdditiveG`) 0.0))
  (:`Released`
    (`AudioParameterControllerInterface.SetTriggerParameter` (`self.AdditiveG`) "Trigger Release")))

(event `Key|F`
  (params (Key :type "Key Structure"))
  (:`Pressed`
    (bind _returnvalue (`GameplayStatics.CreateSound2D` "/Game/Prep/Metasound/MSS_AdditiveSynth.MSS_AdditiveSynth" 1.0 1.0 0.0 null))
    (bind _output_get (set `self.AdditiveB` _returnvalue))
    (`AudioParameterControllerInterface.SetFloatParameter` _output_get "MIDI In" 71.0)
    (`AudioComponent.Play` (`self.AdditiveB`) 0.0))
  (:`Released`
    (`AudioParameterControllerInterface.SetTriggerParameter` (`self.AdditiveB`) "Trigger Release")))

(fn `UserConstructionScript`)