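; MIDI manager Blueprint that plays a polyphonic MetaSound synth from a MIDI controller.
; On BeginPlay it finds the input device matching MIDIControllerIndex and binds its MIDI events.
; Note On spawns an MSS_PolySynth voice stored by note number, shifted up an octave, and Note Off triggers its release.
; Control Change sends the normalized value to voices' Amount parameter; events print on screen, and MonoSynth logic is left unconnected.
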(event `self.ReceiveBeginPlay`
  (bind _outmididevices (`MIDIDeviceManager.FindMIDIDevices`))
  (for _array_element _outmididevices
    (bind (_deviceid _devicename _bcanreceivefrom) (break `FoundMIDIDevice` _array_element))
    (if _bcanreceivefrom
      (if (== (`self.MIDIControllerIndex`) _deviceid)
        (`KismetSystemLibrary.PrintString` _devicename true true (struct :`G` 0.66 :`B` 1.0 :`A` 1.0) 30.0)
        (bind _returnvalue (`MIDIDeviceManager.CreateMIDIDeviceController` _deviceid))
        (bind _output_get (set `self.MIDIControl` _returnvalue))
        (add `MIDIDeviceController.OnMIDIEvent` _output_get (`|CreateDelegate` :!event `EventOnMIDIEvent`)))))
  (`KismetSystemLibrary.PrintString` "BOUCLE TERMINÉE" true true (struct :`G` 0.66 :`B` 1.0 :`A` 1.0) 30.0))

(event `EventOnMIDIEvent`
  (params (MIDIDeviceController :type "MIDIDeviceController Object Reference") (Timestamp :type Integer) (EventType :type "EMIDIEventType Enum" :default "Unknown") (Channel :type Integer) (ControlID :type Integer) (Velocity :type Integer) (RawEventType :type Integer))
  (bind _returnvalue (+ (`KismetMathLibrary.Conv_IntToDouble` ControlID) 12.0))
  (bind _returnvalue_2 (`KismetMathLibrary.FTrunc` _returnvalue))
  ; Imprimer a l'ecran
  (`KismetSystemLibrary.PrintString` (`KismetTextLibrary.Conv_TextToString` (`|FormatText` "MIDI EVENT TYPE {event} MIDI Note {note} VELOCITE {velocite}" ControlID Velocity (`|GetEnumeratorNameAsString` EventType))) true true (struct :`R` 0.022159 :`G` 1.0 :`B` 0.005638 :`A` 1.0) 2.0 "MIDI")
  (switch `EMIDIEventType` EventType
    (:`NoteOff`
      (`AudioParameterControllerInterface.SetTriggerParameter` (`|GetArrayItem` (`self.PolyVoices`) _returnvalue_2) "Trigger Release"))
    (:`NoteOn`
      (bind _returnvalue_3 (`GameplayStatics.CreateSound2D` "/Game/Metasound/MSS_PolySynth.MSS_PolySynth" 1.0 1.0 0.0 null))
      (`KismetArrayLibrary.Array_Set` (`self.PolyVoices`) _returnvalue_2 _returnvalue_3 true)
      (`AudioParameterControllerInterface.SetFloatParameter` _returnvalue_3 "MIDINote" _returnvalue)
      (`AudioComponent.Play` _returnvalue_3 0.0))
    (:`ControlChange`
      (switch `string` (`KismetStringLibrary.Conv_IntToString` ControlID)
        (:`78`
          (for _array_element (`self.PolyVoices`)
            (`/Engine/EditorBlueprintResources/StandardMacros.IsValid` _array_element
              (:`Is Valid`
                (`AudioParameterControllerInterface.SetFloatParameter` _array_element "Amount" (/ (`KismetMathLibrary.Conv_IntToDouble` Velocity) 127.0))))))))))

(fn `UserConstructionScript`)